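; Player character that switches between walking and a rolling armadillo ball, and claws or digs through Destructable actors.
; Holding Armadillo_Mode swaps mesh and capsule for a physics ball and reattaches the spring arm; releasing reverts.
; Movement uses movement input walking and force rolling, with Tick pinning the ball's X to its starting plane.
; Clawing enables the front or, with Digging held, downward hitbox, destroying overlapped Destructables.
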(event OnComponentBeginOverlap(Digging_Hitbox)
  (params (OverlappedComponent :type Primitive%20Component%20Object%20Reference) (OtherActor :type Actor%20Object%20Reference) (OtherComp :type Primitive%20Component%20Object%20Reference) (OtherBodyIndex :type Integer) (bFromSweep :type Boolean) (SweepResult :type Hit%20Result%20Structure%20%28by%20ref%29))
  ;[1 1 1] Destructable Actor Destroy
  (bind _asdestructable (Utilities|Casting|CastToDestructable OtherActor))
  (Actor|DestroyActor _asdestructable))

(event OnComponentBeginOverlap(Front_Claw)
  (params (OverlappedComponent :type Primitive%20Component%20Object%20Reference) (OtherActor :type Actor%20Object%20Reference) (OtherComp :type Primitive%20Component%20Object%20Reference) (OtherBodyIndex :type Integer) (bFromSweep :type Boolean) (SweepResult :type Hit%20Result%20Structure%20%28by%20ref%29))
  ;[1 1 1] Destructable Actor Destroy
  (bind _asdestructable (Utilities|Casting|CastToDestructable OtherActor))
  (Actor|DestroyActor _asdestructable))

(event EventTick
  (params (DeltaSeconds :type Float%20%28single-precision%29))
  (bind _armadillo (Variables|Default|GetArmadillo))
  (bind _returnvalue (Transformation|GetWorldLocation _armadillo))
  (bind (_x _y _z) (Math|Vector|BreakVector _returnvalue))
  ;[1 1 1] Axis Constraining (Holds the character and ball in the Y and Z axis)
  (if (Variables|Default|GetIsAxisConstrained)
    (Transformation|SetWorldLocation _armadillo (Math|Vector|MakeVector (Variables|Default|GetAxisHoldValue) _y _z) false false)))

(event EventBeginPlay
  (bind _armadillo (Variables|Default|GetArmadillo))
  ;[1 1 1] Hide the ball at the beginning
  (Variables|Default|SetIsAxisConstrained true)
  (Variables|Default|SetIsRolled false)
  (Collision|SetCollisionEnabled _armadillo "NoCollision")
  (Physics|SetSimulatePhysics _armadillo false)
  (Development|SetHiddeninGame _armadillo true false)
  (Variables|Default|SetAxisHoldValue (.X (Math|Vector|BreakVector (Transformation|GetWorldLocation (Variables|Collision|GetCapsuleComponent)))))
  ;[1 1 1] Set Triggers to inactive
  (Collision|SetCollisionEnabled (Variables|Default|GetFront_Claw) "NoCollision")
  (Collision|SetCollisionEnabled (Variables|Default|GetDigging_Hitbox) "NoCollision"))

(event Input|ActionEvents|InputActionArmadillo_Mode
  (params (Key :type Key%20Structure))
  (bind _mesh (Variables|Character|GetMesh))
  (bind _capsulecomponent (Variables|Collision|GetCapsuleComponent))
  (bind _armadillo (Variables|Default|GetArmadillo))
  (bind _springarm1 (Variables|Default|GetSpringArm1))
  ;[1 1 1] Transforming to Roll Mode
  (:Pressed
    ;;[1 1 1] Transform to Rolling
    (Variables|Default|SetIsRolled true)
    (CallFunction|SetArmadilloEnabled true)
    (Development|SetHiddeninGame _mesh true false)
    (Collision|SetCollisionEnabled _capsulecomponent "NoCollision")
    (Components|Tick|SetComponentTickEnabled _capsulecomponent false)
    (Transformation|SetWorldLocation _armadillo (Transformation|GetWorldLocation _mesh) false false)
    (Transformation|AttachComponentToComponent _springarm1 _armadillo "None" "SnapToTarget" "KeepRelative" "KeepRelative" true))
  (:Released
    ;;[1 1 1] Revert to Walking
    (Variables|Default|SetIsRolled false)
    (CallFunction|SetArmadilloEnabled false)
    (Development|SetHiddeninGame _mesh false false)
    (Collision|SetCollisionEnabled _capsulecomponent "QueryAndPhysics")
    (Components|Tick|SetComponentTickEnabled _capsulecomponent true)
    (Transformation|SetWorldLocation _capsulecomponent (+ (Transformation|GetWorldLocation _armadillo) "0, 0,10.000000") false false)
    (Transformation|AttachComponentToComponent _springarm1 _capsulecomponent "None" "SnapToTarget" "KeepRelative" "KeepRelative" true)))

(event Input|ActionEvents|InputActionDigging
  (params (Key :type Key%20Structure))
  ;[1 1 1] Setting Down Pressed var
  (:Pressed
    (Variables|Default|SetDownPressed true))
  (:Released
    (Variables|Default|SetDownPressed false)))

(event Input|ActionEvents|InputActionClawing
  (params (Key :type Key%20Structure))
  ;[1 1 1] Clawing and Digging
  (:Pressed
    (if (Variables|Default|GetDownPressed)
      (Collision|SetCollisionEnabled (Variables|Default|GetDigging_Hitbox) "QueryOnly")
      (else
        (Collision|SetCollisionEnabled (Variables|Default|GetFront_Claw) "QueryOnly"))))
  (:Released
    (Collision|SetCollisionEnabled (Variables|Default|GetFront_Claw) "NoCollision")
    (Collision|SetCollisionEnabled (Variables|Default|GetDigging_Hitbox) "NoCollision")))

(event Input|AxisEvents|InputAxisMoveUp
  (params (AxisValue :type Float%20%28single-precision%29))
  ;[1 1 1] Movment
  (if (Variables|Default|GetIsRolled)
    (Physics|AddForce (Variables|Default|GetArmadillo) (* (Math|Vector|Normalize (+ (select (Variables|Default|GetIsAxisConstrained) "0, 0, 0" (* "-1.000000, 0, 0" AxisValue)) (* "0,-1.000000, 0" (stale Input|AxisEvents|InputAxisMoveRight AxisValue)))) (Variables|Default|GetForceMultiplier)) "None" false)
    (else
      (Pawn|Input|AddMovementInput (Math|Vector|Normalize (+ (select (Variables|Default|GetIsAxisConstrained) "0, 0, 0" (* "-1.000000, 0, 0" AxisValue)) (* "0,-1.000000, 0" (stale Input|AxisEvents|InputAxisMoveRight AxisValue)))) 1.0 false))))

(event Input|AxisEvents|InputAxisMoveRight
  (params (AxisValue :type Float%20%28single-precision%29))
  ;[1 1 1] Movment
  (if (Variables|Default|GetIsRolled)
    (Physics|AddForce (Variables|Default|GetArmadillo) (* (Math|Vector|Normalize (+ (select (Variables|Default|GetIsAxisConstrained) "0, 0, 0" (* "-1.000000, 0, 0" (stale Input|AxisEvents|InputAxisMoveUp AxisValue))) (* "0,-1.000000, 0" AxisValue))) (Variables|Default|GetForceMultiplier)) "None" false)
    (else
      (Pawn|Input|AddMovementInput (Math|Vector|Normalize (+ (select (Variables|Default|GetIsAxisConstrained) "0, 0, 0" (* "-1.000000, 0, 0" (stale Input|AxisEvents|InputAxisMoveUp AxisValue))) (* "0,-1.000000, 0" AxisValue))) 1.0 false))))

(fn ConstructionScript
  (Transformation|AttachComponentToComponent (Variables|Default|GetFront_Claw) (Variables|Character|GetMesh) "None" "KeepRelative" "KeepRelative" "KeepRelative" true)
  (Transformation|AttachComponentToComponent (Variables|Default|GetDigging_Hitbox) (Variables|Character|GetMesh) "None" "KeepRelative" "KeepRelative" "KeepRelative" true))

(fn SetArmadilloEnabled
  (params (EnabledState :type Boolean))
  (bind _armadillo (Variables|Default|GetArmadillo))
  (Physics|SetSimulatePhysics _armadillo EnabledState)
  (Development|SetHiddeninGame _armadillo (not EnabledState) false)
  (if EnabledState
    (Collision|SetCollisionEnabled _armadillo (LocalVariables|GetEnabled))
    (else
      (Collision|SetCollisionEnabled _armadillo (LocalVariables|GetDIsabled)))))