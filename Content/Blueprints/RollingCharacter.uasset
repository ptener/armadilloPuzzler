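; Player character that toggles between walking and a physics-simulated Armadillo ball on the Armadillo_Mode input.
; Switching swaps visibility and collision, moves the newly active body to the other's position and reattaches the camera spring arm.
; Movement axes drive walking input or ball torque, with an X-axis constraint for side-on movement.
; Tick pins the ball's X and interpolates camera zoom toward MoveCamera's target; BoostArmadillo's force node is unconnected.
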(event EventTick
  (params (DeltaSeconds :type Float%20%28single-precision%29))
  (bind _springarm1 (Variables|Default|GetSpringArm1))
  (bind _armadillo (Variables|Default|GetArmadillo))
  (bind _returnvalue (Transformation|GetWorldLocation _armadillo))
  (bind (_x _y _z) (Math|Vector|BreakVector _returnvalue))
  ;[1 1 1] Smooth Camera Zooming
  (Variables|/Script/Engine.SpringArmComponent|SetTargetArmLength _springarm1 (Math|Interpolation|FInterpTo (Variables|/Script/Engine.SpringArmComponent|GetTargetArmLength _springarm1) (Variables|Default|GetTargetSpringArmLength) DeltaSeconds (Variables|Default|GetSpringArmInterpSpeed)))
  ;[1 1 1] Axis Constraining (Holds the character and ball in the Y and Z axis)
  (if (Variables|Default|GetIsAxisConstrained)
    (Transformation|SetWorldLocation _armadillo (Math|Vector|MakeVector (Variables|Default|GetAxisHoldValue) _y _z) false false)))

(event EventBeginPlay
  (bind _armadillo (Variables|Default|GetArmadillo))
  ;[1 1 1] Hide the ball at the beginning
  (Variables|Default|SetIsAxisConstrained true)
  (Variables|Default|SetIsRolled false)
  (Collision|SetCollisionEnabled _armadillo "NoCollision")
  (Physics|SetSimulatePhysics _armadillo false)
  (Development|SetHiddeninGame _armadillo true false)
  (Variables|Default|SetAxisHoldValue (.X (Math|Vector|BreakVector (Transformation|GetWorldLocation (Variables|Collision|GetCapsuleComponent))))))

(event Input|ActionEvents|InputActionArmadillo_Mode
  (params (Key :type Key%20Structure))
  (bind _mesh (Variables|Character|GetMesh))
  (bind _capsulecomponent (Variables|Collision|GetCapsuleComponent))
  (bind _armadillo (Variables|Default|GetArmadillo))
  (bind _springarm1 (Variables|Default|GetSpringArm1))
  ;[1 1 1] Transforming to Roll Mode
  (:Released
    (if (Variables|Default|GetIsRolled)
      ;;[1 1 1] Revert to Walking
      (Variables|Default|SetIsRolled false)
      (CallFunction|SetArmadilloEnabled false)
      (Development|SetHiddeninGame _mesh false false)
      (Collision|SetCollisionEnabled _capsulecomponent "QueryAndPhysics")
      (Components|Tick|SetComponentTickEnabled _capsulecomponent true)
      (Transformation|SetWorldLocation _capsulecomponent (+ (Transformation|GetWorldLocation _armadillo) "0, 0,10.000000") false false)
      (Transformation|AttachComponentToComponent _springarm1 _capsulecomponent "None" "SnapToTarget" "KeepRelative" "KeepRelative" true)
      (else
        ;;[1 1 1] Transform to Rolling
        (Variables|Default|SetIsRolled true)
        (CallFunction|SetArmadilloEnabled true)
        (Development|SetHiddeninGame _mesh true false)
        (Collision|SetCollisionEnabled _capsulecomponent "NoCollision")
        (Components|Tick|SetComponentTickEnabled _capsulecomponent false)
        (Transformation|SetWorldLocation _armadillo (Transformation|GetWorldLocation _mesh) false false)
        (Transformation|AttachComponentToComponent _springarm1 _armadillo "None" "SnapToTarget" "KeepRelative" "KeepRelative" true)))))

(event Input|AxisEvents|InputAxisMoveUp
  (params (AxisValue :type Float%20%28single-precision%29))
  ;[1 1 1] Movment
  (if (Variables|Default|GetIsRolled)
    (Class|PrimitiveComponent|AddTorqueinRadians (Variables|Default|GetArmadillo) (* (+ (* "-1.000000, 0, 0" AxisValue) (* "1.000000, 0, 0" (stale Input|AxisEvents|InputAxisMoveRight AxisValue))) (Variables|Default|GetForceMultiplier)) "None" false)
    (else
      (Pawn|Input|AddMovementInput (Math|Vector|Normalize (+ (select (Variables|Default|GetIsAxisConstrained) "0, 0, 0" (* "-1.000000, 0, 0" AxisValue)) (* "0,-1.000000, 0" (stale Input|AxisEvents|InputAxisMoveRight AxisValue)))) 1.0 false))))

(event Input|AxisEvents|InputAxisMoveRight
  (params (AxisValue :type Float%20%28single-precision%29))
  ;[1 1 1] Movment
  (if (Variables|Default|GetIsRolled)
    (Class|PrimitiveComponent|AddTorqueinRadians (Variables|Default|GetArmadillo) (* (+ (* "-1.000000, 0, 0" (stale Input|AxisEvents|InputAxisMoveUp AxisValue)) (* "1.000000, 0, 0" AxisValue)) (Variables|Default|GetForceMultiplier)) "None" false)
    (else
      (Pawn|Input|AddMovementInput (Math|Vector|Normalize (+ (select (Variables|Default|GetIsAxisConstrained) "0, 0, 0" (* "-1.000000, 0, 0" (stale Input|AxisEvents|InputAxisMoveUp AxisValue))) (* "0,-1.000000, 0" AxisValue))) 1.0 false))))

(fn ConstructionScript)

(fn SetArmadilloEnabled
  (params (EnabledState :type Boolean))
  (bind _armadillo (Variables|Default|GetArmadillo))
  (Physics|SetSimulatePhysics _armadillo EnabledState)
  (Development|SetHiddeninGame _armadillo (not EnabledState) false)
  (if EnabledState
    (Collision|SetCollisionEnabled _armadillo (LocalVariables|GetEnabled))
    (else
      (Collision|SetCollisionEnabled _armadillo (LocalVariables|GetDIsabled)))))

(fn BoostArmadillo
  (params (BoostAmount :type Float%20%28single-precision%29) (BoostDirection :type Vector)))

(fn MoveCamera
  (params (TargetArmLength :type Float%20%28single-precision%29) (InterpSpeed :type Float%20%28single-precision%29))
  (Variables|Default|SetTargetSpringArmLength TargetArmLength))